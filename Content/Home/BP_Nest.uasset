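; BP_Nest is a turtle nest that spawns a BP_Turtels at its SpawnVolume whenever its linked Button is pressed.
; After a delay, the Button's display name selects one of three Timelines, which moves the turtle along the Spline from end to start.
; Each variant sets Speed differently, and the third also toggles Movingback.
; On arrival, the turtle plays a pointing montage and is destroyed.
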(event `self.ReceiveBeginPlay`
  (add `/Game/Buttons/BP_Button1.ButPressed` (`self.Button`) (delegate `CustomEvent_0`)))

(event `CustomEvent_0`
  (bind _spline (`self.Spline`))
  (bind _spline_2 (`self.Spline`))
  (bind _spline_3 (`self.Spline`))
  (bind _returnvalue (`|SpawnActorFromClass` "/Game/Turtles/BP_Turtels.BP_Turtels_C" (`SceneComponent.K2_GetComponentToWorld` (`self.SpawnVolume`)) "AlwaysSpawn" "OverrideRootScale" null null))
  (`KismetSystemLibrary.Delay` 2.0)
  (switch `name` (`KismetStringLibrary.Conv_StringToName` (`KismetSystemLibrary.GetDisplayName` (`self.Button`)))
    (:`BP_Button1`
      ;[1 1 1] Логика первой черепашки
      (bind (_direction _turtles1) (`Timeline|Timeline_2` :!via `PlayFromStart`)
        (:`Update`
          (`self.K2_SetActorLocation` _returnvalue (`SplineComponent.GetLocationAtDistanceAlongSpline` _spline (`KismetMathLibrary.Lerp` (`SplineComponent.GetSplineLength` _spline) 0.0 _turtles1) "World") false false)
          (if (== _turtles1 1.0)
            (`Character.PlayAnimMontage` _returnvalue "/Game/Turtles/Models/Pointing_Gesture_mixamo_com_Montage.Pointing_Gesture_mixamo_com_Montage" 1.0 "None")
            (`KismetSystemLibrary.Delay` 2.0)
            (`self.K2_DestroyActor` _returnvalue)))
        (:`Speed`
          (set `/Game/Turtles/BP_Turtels.Speed` 100.0 _returnvalue))))
    (:`BP_Button2`
      ;[1 1 1] Логика второй черепашки
      (bind (_direction_2 _turtles1_2) (`Timeline|Timeline_0` :!via `PlayFromStart`)
        (:`Update`
          (`self.K2_SetActorLocation` _returnvalue (`SplineComponent.GetLocationAtDistanceAlongSpline` _spline_2 (`KismetMathLibrary.Lerp` (`SplineComponent.GetSplineLength` _spline_2) 0.0 _turtles1_2) "World") false false)
          (if (== _turtles1_2 1.0)
            (`Character.PlayAnimMontage` _returnvalue "/Game/Turtles/Models/Pointing_Gesture_mixamo_com_Montage.Pointing_Gesture_mixamo_com_Montage" 1.0 "None")
            (`KismetSystemLibrary.Delay` 2.0)
            (`self.K2_DestroyActor` _returnvalue)))
        (:`Speed1`
          (set `/Game/Turtles/BP_Turtels.Speed` 0.0 _returnvalue))
        (:`Speed2`
          (set `/Game/Turtles/BP_Turtels.Speed` 100.0 _returnvalue))))
    (:`BP_Button3`
      (set `/Game/Turtles/BP_Turtels.bThirdTurtle` true _returnvalue)
      ;[1 1 1] Логика третьей черепашки
      (bind (_direction_3 _turtles1_3) (`Timeline|Timeline_1` :!via `PlayFromStart`)
        (:`Update`
          (set `/Game/Turtles/BP_Turtels.Speed` 100.0 _returnvalue)
          (`self.K2_SetActorLocation` _returnvalue (`SplineComponent.GetLocationAtDistanceAlongSpline` _spline_3 (`KismetMathLibrary.Lerp` (`SplineComponent.GetSplineLength` _spline_3) 0.0 _turtles1_3) "World") false false)
          (if (== _turtles1_3 1.0)
            (`Character.PlayAnimMontage` _returnvalue "/Game/Turtles/Models/Pointing_Gesture_mixamo_com_Montage.Pointing_Gesture_mixamo_com_Montage" 1.0 "None")
            (`KismetSystemLibrary.Delay` 2.0)
            (`self.K2_DestroyActor` _returnvalue)))
        (:`NewTrack_0`
          (set `/Game/Turtles/BP_Turtels.bMovingback` true _returnvalue))
        (:`NewTrack_1`
          (set `/Game/Turtles/BP_Turtels.bMovingback` false _returnvalue))))))

(fn `UserConstructionScript`)